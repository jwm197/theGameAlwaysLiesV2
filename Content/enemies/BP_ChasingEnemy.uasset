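; Side-scroller enemy that patrols along X, then chases the player in X and Z, killing on overlap if CanKill is set.
; BeginPlay detaches and hides markers P1 and P2 to fix patrol bounds, and disables collision on non-killing enemies.
; Tick moves it by unswept local offsets, flipping rotation 180 degrees to change direction.
; AIPerception ends patrolling on sensing the player, and nothing here resumes it.
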(event OnTargetPerceptionUpdated(AIPerception)
  (params (Actor :type Actor%20Object%20Reference) (Stimulus :type AI%20Stimulus%20Structure))
  (Utilities|Casting|CastToplayer Actor)
  (if (.bSuccessfullySensed (Utilities|Struct|BreakAIStimulus Stimulus))
    (Variables|Default|SetPatrolling false)))

(event EventBeginPlay
  (Transformation|DetachFromComponent (Variables|Default|Getp1) "KeepWorld" "KeepWorld" "KeepWorld" true)
  (Variables|/Script/Engine.CharacterMovementComponent|SetMaxWalkSpeed (Variables|Character|GetCharacterMovement) (Variables|Default|GetMax%20Walk%20Speed))
  (Variables|Default|SetAIPosition (.x (Transformation|GetActorLocation)))
  (Variables|Default|SetStartPosition (- (.x (Transformation|GetSocketLocation (Variables|Default|Getp2) "None")) (Variables|Default|GetAIPosition)))
  (Variables|Default|SetEndPosition (- (.x (Transformation|GetSocketLocation (Variables|Default|Getp1) "None")) (Variables|Default|GetAIPosition)))
  (Rendering|SetVisibility (Variables|Default|Getp1) false false)
  (if (not (Variables|Default|GetCanKill))
    (Collision|SetCollisionEnabled (Variables|Collision|GetCapsuleComponent) "NoCollision")))

(event Collision|EventActorBeginOverlap
  (params (OtherActor :type Actor%20Object%20Reference))
  (bind _asplayer (Utilities|Casting|CastToplayer OtherActor))
  (if (Variables|Default|GetCanKill)
    (Default|Killplayer _asplayer)))

(event EventTick
  (params (DeltaSeconds :type Float%20%28single-precision%29))
  (bind _returnvalue (Transformation|GetActorLocation))
  (Variables|Default|SetAIMovingPositionX (.x _returnvalue))
  (Variables|Default|SetALMovingPositionZ (.z _returnvalue))
  (if (Variables|Default|GetPatrolling)
    (|PatrollingNode)
    (elif (> (.x (Transformation|GetActorLocation (Game|GetPlayerCharacter 0))) (Variables|Default|GetAIMovingPositionX))
      (|Playeronrightside)
      (else
        (|Playeronleftside)))))

(fn ConstructionScript)